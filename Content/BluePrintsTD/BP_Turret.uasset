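; BP_Turret is a tower-defense turret that automatically aims and fires at BP_Enemy pawns it sees.
; Each PawnSensing sighting swings RotateBall toward the enemy with a short MoveComponentTo, using only look-at yaw and roll, without pitch.
; It then spawns a BP_Bullet at the Arrow component's transform and plays a pop sound.
; The graph has no timer or cooldown, so sighting events drive the firing.
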(event `self.ReceiveTick`
  (params (DeltaSeconds :type "Float (single-precision)")))

(event `self.PawnSensing.OnSeePawn`
  (params (Pawn :type "Pawn Object Reference"))
  (bind _asbp_enemy (cast `/Game/BluePrintsTD/BP_Enemy` Pawn))
  (`|ExecutionSequence`
    (:`then_0`
      (bind (_returnvalue_roll _returnvalue_pitch _returnvalue_yaw) (`KismetMathLibrary.BreakRotator` (`KismetMathLibrary.FindLookAtRotation` (`self.K2_GetActorLocation`) (`self.K2_GetActorLocation` _asbp_enemy))))
      (`KismetSystemLibrary.MoveComponentTo` (`self.RotateBall`) (0.0 0.0 0.0) (`KismetMathLibrary.MakeRotator` _returnvalue_roll 0.0 _returnvalue_yaw) false false 0.06)
      (`|SpawnActorFromClass` "/Game/BluePrintsTD/BP_Bullet.BP_Bullet_C" (`SceneComponent.K2_GetComponentToWorld` (`self.Arrow`)) "Undefined" "MultiplyWithRoot" null null)
      (`GameplayStatics.PlaySoundAtLocation` "/Game/Sound/Interface_And_Item_Sounds/Cues/Pop_02_Cue.Pop_02_Cue" (`self.K2_GetActorLocation`) (struct) 1.0 1.0 0.0 null null null null))))

(fn `UserConstructionScript`)