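; BP_Base is the tower-defense base that enemies attack, tracking its health from a starting value set at BeginPlay.
; A one-time Tick step caches the third-person player character and initializes the health display in its main UI.
; Enemies overlapping the Box subtract their base damage, then die and update the UI while health remains.
; At zero health it triggers the player's GameOver and destroys itself with an explosion effect and sound.
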(event `self.ReceiveBeginPlay`
  (set `self.BaseHPCurrent` (`self.BaseHP`)))

(event `self.ReceiveTick`
  (params (DeltaSeconds :type "Float (single-precision)"))
  (`/Engine/EditorBlueprintResources/StandardMacros.DoOnce` false
    (:`Completed`
      (bind _asbp_third_person_character (cast `/Game/ThirdPerson/Blueprints/BP_ThirdPersonCharacter` (`GameplayStatics.GetPlayerCharacter` 0)))
      (`/Game/UI/WB_Main.SetBaseHealthInfo` (`/Game/ThirdPerson/Blueprints/BP_ThirdPersonCharacter.MainUi` _asbp_third_person_character) (`KismetMathLibrary.FTrunc` (`self.BaseHp`))))))

(event `self.Box.OnComponentBeginOverlap`
  (params (OverlappedComponent :type "PrimitiveComponent Object Reference") (OtherActor :type "Actor Object Reference") (OtherComp :type "PrimitiveComponent Object Reference") (OtherBodyIndex :type Integer) (bFromSweep :type Boolean) (SweepResult :type "HitResult Structure (by ref)"))
  (bind _returnvalue (`self.K2_GetActorLocation`))
  (bind _asbp_enemy (cast `/Game/BluePrintsTD/BP_Enemy` OtherActor))
  (bind _output_get (set `self.BaseHpCurrent` (- (`self.BaseHpCurrent`) (`/Game/BluePrintsTD/BP_Enemy.DamageToBase` _asbp_enemy))))
  (if (<= _output_get 0.0)
    (`/Game/ThirdPerson/Blueprints/BP_ThirdPersonCharacter.GameOver` (stale `self.ReceiveTick` _asbp_third_person_character))
    (`self.K2_DestroyActor`)
    (`GameplayStatics.SpawnEmitterAtLocation` "/Game/Realistic_Starter_VFX_Pack_Vol2/Particles/Explosion/P_Explosion_Big_C.P_Explosion_Big_C" _returnvalue (struct) (10.0 10.0 10.0))
    (`GameplayStatics.PlaySoundAtLocation` "/Game/Starter/StarterContent/Audio/Explosion_Cue.Explosion_Cue" _returnvalue (struct) 1.0 1.0 0.0 null null null null)
    (else
      (`/Game/BluePrintsTD/BP_Enemy.Die` _asbp_enemy)
      (`/Game/UI/WB_Main.SetBaseHealthInfo` (`/Game/ThirdPerson/Blueprints/BP_ThirdPersonCharacter.MainUi` (stale `self.ReceiveTick` _asbp_third_person_character)) (`KismetMathLibrary.FTrunc` (`self.BaseHpCurrent`))))))

(fn `UserConstructionScript`)