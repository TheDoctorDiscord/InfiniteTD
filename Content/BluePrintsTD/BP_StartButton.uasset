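; BP_StartButton is an interactable button that starts an enemy wave in what appears to be a tower defense game.
; A sphere overlap by BP_ThirdPersonCharacter enables input and opens a gate, and leaving reverses both.
; IA_Interact passes through the gate and a DoOnce, so only the first press calls StartWave on the first BP_SpawnPoint found and WaveProgress on the character's MainUi.
; A StopWave branch is left unconnected.
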(event `EnhancedInput|/Game/ThirdPerson/Input/Actions/IA_Interact`
  (params (ActionValue :type Boolean) (ElapsedSeconds :type "Float (double-precision)") (TriggeredSeconds :type "Float (double-precision)") (InputAction :type "InputAction Object Reference" :default "/Game/ThirdPerson/Input/Actions/IA_Interact.IA_Interact"))
  (:`Started`
    (`/Engine/EditorBlueprintResources/StandardMacros.Gate` true :!label _label
      (:`Exit`
        (bind _outactors (`GameplayStatics.GetAllActorsOfClass` "/Game/BluePrintsTD/BP_SpawnPoint.BP_SpawnPoint_C"))
        (`/Engine/EditorBlueprintResources/StandardMacros.DoOnce` false
          (:`Completed`
            (`/Game/BluePrintsTD/BP_SpawnPoint.StartWave` (`|GetArrayItem` _outactors))
            (`/Game/UI/WB_Main.WaveProgress` (`/Game/ThirdPerson/Blueprints/BP_ThirdPersonCharacter.MainUi` (stale `self.Sphere.OnComponentBeginOverlap` _asbp_third_person_character)))))))))

(event `self.Sphere.OnComponentBeginOverlap`
  (params (OverlappedComponent :type "PrimitiveComponent Object Reference") (OtherActor :type "Actor Object Reference") (OtherComp :type "PrimitiveComponent Object Reference") (OtherBodyIndex :type Integer) (bFromSweep :type Boolean) (SweepResult :type "HitResult Structure (by ref)"))
  (bind _asbp_third_person_character (cast `/Game/ThirdPerson/Blueprints/BP_ThirdPersonCharacter` OtherActor))
  (`self.EnableInput` (`GameplayStatics.GetPlayerController` 0))
  (goto _label :!via `Open`))

(event `self.Sphere.OnComponentEndOverlap`
  (params (OverlappedComponent :type "PrimitiveComponent Object Reference") (OtherActor :type "Actor Object Reference") (OtherComp :type "PrimitiveComponent Object Reference") (OtherBodyIndex :type Integer))
  (cast `/Game/ThirdPerson/Blueprints/BP_ThirdPersonCharacter` OtherActor)
  (`self.DisableInput` (`GameplayStatics.GetPlayerController` 0))
  (goto _label :!via `Close`))

(fn `UserConstructionScript`)