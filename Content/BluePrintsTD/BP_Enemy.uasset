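; BP_Enemy is a tower-defense enemy that walks to the first TargetPoint found and explodes on arrival.
; Its random eye material doubles as hit points: each damage event, regardless of amount, steps it down one tier in ArrayMat.
; A hit at the lowest tier pays RewardMoney, randomly multiplied at spawn independently of tier, to the player's BPCBuildSystem and destroys it.
; Die explodes it without reward; the Health-based damage logic is disconnected.
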(event `self.ReceiveBeginPlay`
  (bind _returnvalue (`KismetMathLibrary.RandomIntegerInRange` 0 2))
  (bind _returnvalue_2 (`self.K2_GetActorLocation`))
  (`PrimitiveComponent.SetMaterial` (`self.Eye`) 0 (`|GetArrayItem` (`self.ArrayMat`) _returnvalue))
  (`PrimitiveComponent.SetMaterial` (`self.EyeColor`) 0 (`PrimitiveComponent.GetMaterial` (`self.Eye`) 0))
  (set `self.RewardMoney` (* (`self.RewardMoney`) (+ _returnvalue 1)))
  (`KismetSystemLibrary.Delay` 0.2)
  (bind _outactors (`GameplayStatics.GetAllActorsOfClass` "/Script/Engine.TargetPoint"))
  (`|AIMoveTo` self (0.0 0.0 0.0) (`|GetArrayItem` _outactors) 1.0
    (:`OnSuccess`
      (`GameplayStatics.SpawnEmitterAtLocation` "/Game/Starter/StarterContent/Particles/P_Explosion.P_Explosion" _returnvalue_2)
      (`GameplayStatics.PlaySoundAtLocation` "/Game/Sound/Sound_effects_Mini_Pack1_5/Explosions/WAV/Explosion1_Cue.Explosion1_Cue" _returnvalue_2 (struct) 1.0 1.0 0.0 null null null null)
      (`self.K2_DestroyActor`))))

(event `Die`
  (bind _returnvalue (`self.K2_GetActorLocation`))
  (`GameplayStatics.SpawnEmitterAtLocation` "/Game/Starter/StarterContent/Particles/P_Explosion.P_Explosion" _returnvalue)
  (`GameplayStatics.PlaySoundAtLocation` "/Game/Sound/Sound_effects_Mini_Pack1_5/Explosions/WAV/Explosion1_Cue.Explosion1_Cue" _returnvalue (struct) 1.0 1.0 0.0 null null null null)
  (`self.K2_DestroyActor`))

(event `self.ReceiveAnyDamage`
  (params (Damage :type "Float (single-precision)") (DamageType :type "DamageType Object Reference") (InstigatedBy :type "Controller Object Reference") (DamageCauser :type "Actor Object Reference"))
  (bind _returnvalue (`self.K2_GetActorLocation`))
  (bind _arraymat (`self.ArrayMat`))
  (bind _eye (`self.Eye`))
  (bind _eyecolor (`self.EyeColor`))
  (bind _returnvalue_2 (`PrimitiveComponent.GetMaterial` (`self.Eye`) 0))
  (if (== (`PrimitiveComponent.GetMaterial` _eye 0) (`|GetArrayItem` _arraymat 2))
    (`PrimitiveComponent.SetMaterial` _eye 0 (`|GetArrayItem` (`self.ArrayMat`) 1))
    (`PrimitiveComponent.SetMaterial` _eyecolor 0 _returnvalue_2)
    (elif (== (`PrimitiveComponent.GetMaterial` _eye 0) (`|GetArrayItem` _arraymat 1))
      (`PrimitiveComponent.SetMaterial` _eye 0 (`|GetArrayItem` (`self.ArrayMat`)))
      (`PrimitiveComponent.SetMaterial` _eyecolor 0 _returnvalue_2)
      (elif (== (`PrimitiveComponent.GetMaterial` _eye 0) (`|GetArrayItem` _arraymat))
        (bind _asbp_third_person_character (cast `/Game/ThirdPerson/Blueprints/BP_ThirdPersonCharacter` (`GameplayStatics.GetPlayerCharacter` 0)))
        (`/Game/ThirdPerson/Blueprints/BPC_BuildSystem.IncreaseMoney` (`/Game/ThirdPerson/Blueprints/BP_ThirdPersonCharacter.BPC_BuildSystem` _asbp_third_person_character) (`self.RewardMoney`))
        (`GameplayStatics.SpawnEmitterAtLocation` "/Game/Starter/StarterContent/Particles/P_Explosion.P_Explosion" _returnvalue)
        (`GameplayStatics.PlaySoundAtLocation` "/Game/Sound/Sound_effects_Mini_Pack1_5/Explosions/WAV/Explosion1_Cue.Explosion1_Cue" _returnvalue (struct) 1.0 1.0 0.0 null null null null)
        (`self.K2_DestroyActor`)))))

(fn `UserConstructionScript`)