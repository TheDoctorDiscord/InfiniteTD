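; Tower defense spawn point that releases a wave of BP_Enemy pawns and triggers the win when none remain.
; StartWave runs a delayed, breakable loop spawning enemies with electric effect and sound at the Sphere, reducing SpawnRate each spawn, while StopWave breaks it.
; Starting a wave also enables a delay-throttled Tick check that calls GameWon on the player character when no valid enemy is found.
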(event `StartWave`
  (bind _returnvalue (`SceneComponent.K2_GetComponentLocation` (`self.Sphere`)))
  (bind _returnvalue_2 (+ _returnvalue (0.0 0.0 20.0)))
  (`|ExecutionSequence`
    (:`then_0`
      (`/Game/BluePrintsTD/BPM_Library.For Loop With Delay And Break` 0 (`self.EnemySpawnAmount`) (`self.SpawnRate`) :!label _label
        (:`Loop Body`
          (set `self.SpawnRate` (- (`self.SpawnRate`) 0.02))
          (`AIBlueprintHelperLibrary.SpawnAIFromClass` "/Game/BluePrintsTD/BP_Enemy.BP_Enemy_C" null _returnvalue (`SceneComponent.K2_GetComponentRotation` (`self.Sphere`)) false null)
          (`GameplayStatics.SpawnEmitterAtLocation` "/Game/Realistic_Starter_VFX_Pack_Vol2/Particles/Destruction/P_Destruction_Electric.P_Destruction_Electric" _returnvalue_2)
          (`GameplayStatics.PlaySoundAtLocation` "/Game/Sound/Interface_And_Item_Sounds/Cues/Futuristic_Click_07_Cue.Futuristic_Click_07_Cue" _returnvalue_2 (struct) 1.0 1.0 0.0 null null null null))))
    (:`then_1`
      (set `self.CheckMode` true))))

(event `StopWave`
  (goto _label :!via `Break`))

(event `self.ReceiveTick`
  (params (DeltaSeconds :type "Float (single-precision)"))
  (if (`self.CheckMode`)
    (`KismetSystemLibrary.Delay` 2.0)
    (bind _returnvalue (`GameplayStatics.GetActorOfClass` "/Game/BluePrintsTD/BP_Enemy.BP_Enemy_C"))
    (`/Engine/EditorBlueprintResources/StandardMacros.IsValid` _returnvalue
      (:`Is Not Valid`
        (bind _asbp_third_person_character (cast `/Game/ThirdPerson/Blueprints/BP_ThirdPersonCharacter` (`GameplayStatics.GetPlayerCharacter` 0)))
        (`/Game/ThirdPerson/Blueprints/BP_ThirdPersonCharacter.GameWon` _asbp_third_person_character)))))

(event `self.ReceiveBeginPlay`)

(fn `UserConstructionScript`)