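; BP_Bullet is a short-lived projectile actor that deals damage on impact.
; When its Sphere component hits, it applies its damage and damage type to the hit actor, crediting its owner, and spawns an impact particle and sound.
; The hit does not destroy the bullet; it destroys itself when the projectile movement bounces or half a second after spawning.
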(event `self.ReceiveBeginPlay`
  (`KismetSystemLibrary.Delay` 0.5)
  (`self.K2_DestroyActor`))

(event `self.ProjectileMovement.OnProjectileBounce`
  (params (ImpactResult :type "HitResult Structure (by ref)") (ImpactVelocity :type "Vector Structure (by ref)"))
  (`self.K2_DestroyActor`))

(event `self.Sphere.OnComponentHit`
  (params (HitComponent :type "PrimitiveComponent Object Reference") (OtherActor :type "Actor Object Reference") (OtherComp :type "PrimitiveComponent Object Reference") (NormalImpulse :type "Vector Structure") (Hit :type "HitResult Structure (by ref)"))
  (bind _returnvalue (`self.K2_GetActorLocation`))
  (`GameplayStatics.ApplyDamage` OtherActor (`self.Damage`) null (`self.GetOwner`) "/Script/Engine.DamageType")
  (`GameplayStatics.SpawnEmitterAtLocation` "/Game/Realistic_Starter_VFX_Pack_Vol2/Particles/Hit/P_Default.P_Default" _returnvalue (struct) (0.8 0.8 0.8))
  (`GameplayStatics.PlaySoundAtLocation` "/Game/Sound/Sound_effects_Mini_Pack1_5/Hit/WAV/Hit3_Cue.Hit3_Cue" _returnvalue (struct) 1.0 1.0 0.0 null null null null))

(fn `UserConstructionScript`)